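; Spawner actor that builds a chain of BP_Tunnel segments and populates them with enemies and health packs.
; On BeginPlay it destroys existing tunnels, then starts a short run at the player pawn, attaching each next segment at the newest one's SpawnPoint.
; Each segment receives a spawner reference and a randomized wall.
; Randomly offset pickups and enemies spawn ahead: health packs by coin flip, enemies always, since their random roll is fixed.
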(event `self.ReceiveBeginPlay`
  (`self.SpawnInitialTunnels`))

(fn `SpawnEnemy`
  (params (`Spawn Location` :type "Vector Structure"))
  (if (== (`KismetMathLibrary.RandomIntegerInRange` 0) 0)
    (`|SpawnActorFromClass` "/Game/InfiniteMatrix/Blueprints/BP_Enemy.BP_Enemy_C" (`KismetMathLibrary.MakeTransform` `Spawn Location`) "Undefined" "MultiplyWithRoot" null null)))

(fn `SpawnEntities`
  (params (SpawnLocation :type "Vector Structure"))
  (bind _returnvalue (+ SpawnLocation (`KismetMathLibrary.MakeVector` 1200.0 (`KismetMathLibrary.Conv_IntToDouble` (`KismetMathLibrary.RandomIntegerInRange` -150 150)) (`KismetMathLibrary.Conv_IntToDouble` (`KismetMathLibrary.RandomIntegerInRange` -150 150)))))
  (`|ExecutionSequence`
    (:`then_0`
      (bind _returnvalue_2 (`|SpawnActorFromClass` "/Game/InfiniteMatrix/Blueprints/BP_Tunnel.BP_Tunnel_C" (`KismetMathLibrary.MakeTransform` SpawnLocation) "Undefined" "MultiplyWithRoot" null null))
      (bind _output_get (set `self.NewestTunnel` _returnvalue_2))
      (set `/Game/InfiniteMatrix/Blueprints/BP_Tunnel.TunnelSpawner` self _output_get)
      (`/Game/InfiniteMatrix/Blueprints/BP_Tunnel.RandomizeWall` _output_get))
    (:`then_1`
      (`self.SpawnHealthPack` _returnvalue)
      (`self.SpawnEnemy` (+ _returnvalue (`KismetMathLibrary.MakeVector` 600.0 (`KismetMathLibrary.Conv_IntToDouble` (`KismetMathLibrary.RandomIntegerInRange` -150 150)) (`KismetMathLibrary.Conv_IntToDouble` (`KismetMathLibrary.RandomIntegerInRange` -150 150))))))))

(fn `SpawnHealthPack`
  (params (`Spawn Location` :type "Vector Structure"))
  (if (== (`KismetMathLibrary.RandomIntegerInRange` 0 1) 0)
    (`|SpawnActorFromClass` "/Game/InfiniteMatrix/Blueprints/BP_HealthPack.BP_HealthPack_C" (`KismetMathLibrary.MakeTransform` `Spawn Location`) "Undefined" "MultiplyWithRoot" null null)))

(fn `SpawnInitialTunnels`
  (`|ExecutionSequence`
    (:`then_0`
      (bind _outactors (`GameplayStatics.GetAllActorsOfClass` "/Game/InfiniteMatrix/Blueprints/BP_Tunnel.BP_Tunnel_C"))
      (for _array_element _outactors
        (`self.K2_DestroyActor` _array_element)))
    (:`then_1`
      (for _ (range 3)
        (`/Engine/EditorBlueprintResources/StandardMacros.IsValid` (`self.NewestTunnel`)
          (:`Is Valid`
            (`self.SpawnTunnelAtSpawnPoint`))
          (:`Is Not Valid`
            (`self.SpawnEntities` (`self.K2_GetActorLocation` (`GameplayStatics.GetPlayerPawn` 0)))))))))

(fn `SpawnTunnelAtSpawnPoint`
  (`self.SpawnEntities` (`SceneComponent.K2_GetComponentLocation` (`/Game/InfiniteMatrix/Blueprints/BP_Tunnel.SpawnPoint` (`self.NewestTunnel`)))))

(fn `UserConstructionScript`)