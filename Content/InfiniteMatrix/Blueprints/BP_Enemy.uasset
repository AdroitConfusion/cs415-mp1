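; BP_Enemy is an enemy actor that damages the player on contact and awards score when shot.
; An EnemyMesh overlap with BP_Player decrements health, while one with BP_Projectile increments player 0's Score and destroys the projectile; both destroy the enemy.
; A blocking hit from a projectile destroys only the enemy, without scoring.
; A Delay on Tick, rather than BeginPlay, limits its lifetime to 15 seconds.
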(event `self.ReceiveTick`
  (params (DeltaSeconds :type "Float (single-precision)"))
  (`KismetSystemLibrary.Delay` 15.0)
  (`self.K2_DestroyActor`))

(event `self.EnemyMesh.OnComponentBeginOverlap`
  (params (OverlappedComponent :type "PrimitiveComponent Object Reference") (OtherActor :type "Actor Object Reference") (OtherComp :type "PrimitiveComponent Object Reference") (OtherBodyIndex :type Integer) (bFromSweep :type Boolean) (SweepResult :type "HitResult Structure (by ref)"))
  (`|ExecutionSequence`
    (:`then_0`
      (bind _asbp_player (cast `/Game/InfiniteMatrix/Blueprints/BP_Player` OtherActor))
      (`/Game/InfiniteMatrix/Blueprints/BP_Player.DecrementHealth` _asbp_player)
      (`self.K2_DestroyActor`))
    (:`then_1`
      (bind _asbp_projectile (cast `/Game/InfiniteMatrix/Blueprints/BP_Projectile` OtherActor))
      (bind _asbp_player_2 (cast `/Game/InfiniteMatrix/Blueprints/BP_Player` (`GameplayStatics.GetPlayerPawn` 0)))
      (`/Engine/EditorBlueprintResources/StandardMacros.IncrementFloat` (`/Game/InfiniteMatrix/Blueprints/BP_Player.score` _asbp_player_2)
        (:`  `
          (`self.K2_DestroyActor` _asbp_projectile)
          (`self.K2_DestroyActor`))))))

(event `self.EnemyMesh.OnComponentHit`
  (params (HitComponent :type "PrimitiveComponent Object Reference") (OtherActor :type "Actor Object Reference") (OtherComp :type "PrimitiveComponent Object Reference") (NormalImpulse :type "Vector Structure") (Hit :type "HitResult Structure (by ref)"))
  (cast `/Game/InfiniteMatrix/Blueprints/BP_Projectile` OtherActor)
  (`self.K2_DestroyActor`))

(fn `UserConstructionScript`)